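; Widget component for BP_Painting_Base actors that hands the painting's data to its UI widget.
; The custom FakePre-Construction event caches the owning painting, pushes its PaintingData into the WWBP_Base widget, then resets the component to StartingRelativeTransform.
; SaveStartingTransform records that relative transform through a DoOnce, and nothing in this graph calls it.
; BeginPlay and Tick are empty.
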(event Custom|Fake%20Pre-Construction
  (Utilities|FlowControl|Sequence
    (:then_1
      (bind _asbp_painting_base (Utilities|Casting|CastToBP_Painting_Base (Components|GetOwner)))
      (Variables|Default|SetParent%20Painting _asbp_painting_base)
      (CallFunction|RetrievePaintingDatafromParent)
      (Transformation|SetRelativeTransform (Variables|Default|GetStartingRelativeTransform) false true))))

(event Custom|SaveStartingTransform
  (Utilities|FlowControl|DoOnce false
    (:Completed
      (Variables|Default|SetStartingRelativeTransform (Transformation|GetRelativeTransform)))))

(event EventBeginPlay)

(event EventTick
  (params (DeltaSeconds :type Float%20%28single-precision%29)))

(fn RetrievePaintingDatafromParent
  (bind _aswwbp_base (Utilities|Casting|CastToWWBP_Base (UserInterface|GetUserWidgetObject)))
  (Default|SetPaintingData _aswwbp_base (Variables|/PublicContent/BP_Painting_Base.BP_Painting_Base_C|GetPaintingData (Variables|Default|GetParent%20Painting))))