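; Base painting actor that displays a picture on a canvas scaled to its real size in centimetres, with attached painting widgets.
; Construct runs in editor and at BeginPlay, applying PaintingData through a dynamic material and refreshing widgets.
; Size and texture setters update PaintingData and fire change dispatchers; resizing re-offsets widgets from saved starting transforms in proportion to canvas size.
; Textures set before the material exists are cached and retried on Tick.
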(event Custom|Обновить%20текст%20и%20портрет
  (bind _paintingdata (Variables|Default|GetPaintingData))
  (bind _painting_widget (Utilities|ForEachWPaintingWidget)
    (:LoopBody
      (Default|FakePre-Construction _painting_widget))
    (:Completed
      (CallFunction|SetCanvasSizeandTexture (.realsize _paintingdata) (.picture _paintingdata) false)
      (CallFunction|UpdateWidgetsShift))))

(event Custom|OnCanvasResize
  (params (New%20SIze%20cm :type Vector%202D%20Structure))
  (CallFunction|UpdateWidgetsShift)
  (Development|PrintString (Utilities|String|ToString(Vector2d) New%20SIze%20cm)))

(event EventBeginPlay
  (CallFunction|Construct)
  (EventDispatchers|BindEventtoOnCanvasSizeChanged (delegate Custom|OnCanvasResize)))

(event Collision|EventActorBeginOverlap
  (params (OtherActor :type Actor%20Object%20Reference)))

(event EventTick
  (params (DeltaSeconds :type Float%20%28single-precision%29))
  ;[1 1 1] Delayed canvas texture setup
  (Utilities|IsValid (Variables|Delayedtexture|GetDelayed%20Texture)
    (:Is%20Valid
      (bind _success (CallFunction|SetCanvasTexture (Variables|Delayedtexture|GetDelayed%20Texture) (Variables|DelayedTexture|GetShow%20Canvas%20On%20Success)))
      (if _success
        (Variables|Delayedtexture|SetDelayed%20Texture 0)))))

(fn ConstructionScript
  (bind _painting_widget (Utilities|ForEachWPaintingWidget)
    (:LoopBody
      (Default|SaveStartingTransform _painting_widget))
    (:Completed
      (CallFunction|Construct))))

(fn GetPaintingData
  (return (Variables|Default|GetPaintingData)))

(fn Construct
  (Utilities|FlowControl|Sequence
    (:then_2
      ;[1 1 1] Canvas Setup
      ;;[1 0.6112 0] TODO CHECK VALIDITY?
      (if true
        (CallFunction|SetCanvasSize (Utilities|Struct|BreakST_PaintingData (CallFunction|GetPaintingData)))
        (bind _returnvalue (Rendering|Material|CreateDynamicMaterialInstance (Variables|Default|GetCanvas) 0 "/PublicContent/M_Painting_Base.M_Painting_Base" "None" :!class /Script/Engine.PrimitiveComponent))
        (Variables|Internal|SetCanvas%20Dynamic%20Material%20Instance _returnvalue)
        (CallFunction|SetCanvasTexture (Utilities|Struct|BreakST_PaintingData (Variables|Default|GetPaintingData)) false)))
    (:then_3
      (bind _painting_widget (Utilities|ForEachWPaintingWidget)
        (:LoopBody
          (Utilities|FlowControl|Sequence
            (:then_1
              (Default|FakePre-Construction _painting_widget))))
        (:Completed
          (CallFunction|UpdateWidgetsShift))))))

(fn SetCanvasSize
  (params (New%20Size%20cm :type Vector%202D%20Structure))
  (bind (_x _y) (Math|Vector2D|BreakVector2D New%20Size%20cm))
  (Transformation|SetRelativeScale3D (Variables|Default|GetCanvas) (Math|Vector|MakeVector (* _x 0.01) (* _y 0.01) 1.0))
  (bind _output_get (LocalVariables|SetCanvasSizeDifferent (Math|Vector|Equal(Vector) (Utilities|Struct|BreakST_PaintingData (Variables|Default|GetPaintingData)) New%20Size%20cm 0.0001)))
  (if (not _output_get)
    (Utilities|Struct|SetmembersinST_PaintingData (Variables|Default|GetPaintingData) New%20Size%20cm)
    (Default|CallOnCanvasSizeChanged New%20Size%20cm)))

(fn SetCanvasTexture
  (params (New%20Texture :type Texture%202D%20Object%20Reference) (Show%20Canvas%20on%20success :type Boolean))
  (bind _canvas_dynamic_material_instance (Variables|Internal|GetCanvas%20Dynamic%20Material%20Instance))
  (Utilities|IsValid _canvas_dynamic_material_instance
    (:Is%20Valid
      (Rendering|Material|SetTextureParameterValue _canvas_dynamic_material_instance "Texture" New%20Texture)
      (if Show%20Canvas%20on%20success
        (Development|SetHiddeninGame (Variables|Default|GetCanvas) false false))
      (if (== New%20Texture (Utilities|Struct|BreakST_PaintingData (Variables|Default|GetPaintingData))) ; Если текстура другая
        _
        (else
          (Utilities|Struct|SetmembersinST_PaintingData (Variables|Default|GetPaintingData) New%20Texture)
          (Default|CallOnCanvasTextureChanged New%20Texture)))
      (return true))
    (:Is%20Not%20Valid
      (Variables|Delayedtexture|SetDelayed%20Texture New%20Texture)
      (Variables|DelayedTexture|SetShow%20Canvas%20On%20Success Show%20Canvas%20on%20success)
      (return false))))

(fn SetCanvasSizeandTexture
  (params (New%20Size%20cm :type Vector%202D%20Structure) (New%20Texture :type Texture%202D%20Object%20Reference) (Show%20Canvas%20on%20Texture%20success :type Boolean))
  (Utilities|FlowControl|Sequence
    (:then_0
      (if (not (Math|Vector|Equal(Vector) :A New%20Size%20cm))
        (CallFunction|SetCanvasSize New%20Size%20cm)))
    (:then_1
      (Utilities|IsValid New%20Texture
        (:Is%20Valid
          (CallFunction|SetCanvasTexture New%20Texture Show%20Canvas%20on%20Texture%20success))))))

(fn UpdateWidgetsShift
  ;[1 1 1] Widgets Shift
  (for _array_element (Actor|GetComponentsByClass "/PublicContent/BP_Painting_Widget_Component.BP_Painting_Widget_Component_C")
    (Transformation|SetRelativeTransform _array_element (Math|Transform|ComposeTransforms (Variables|/PublicContent/BP_Painting_Widget_Component.BP_Painting_Widget_Component_C|GetStartingRelativeTransform _array_element) (Math|Transform|MakeTransform (Math|Vector|MakeVector 0.0 (.x (* (Variables|/PublicContent/BP_Painting_Widget_Component.BP_Painting_Widget_Component_C|GetPainting%20Shift _array_element) (Utilities|Struct|BreakST_PaintingData (CallFunction|GetPaintingData)) "(X=-1.000000,Y=1.000000)")) (.y (* (Variables|/PublicContent/BP_Painting_Widget_Component.BP_Painting_Widget_Component_C|GetPainting%20Shift _array_element) (Utilities|Struct|BreakST_PaintingData (CallFunction|GetPaintingData)) "(X=-1.000000,Y=1.000000)"))))) false true)))